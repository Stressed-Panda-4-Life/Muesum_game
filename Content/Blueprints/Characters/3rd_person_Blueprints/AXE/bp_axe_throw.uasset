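; Thrown axe actor that launches from the player, deals damage on impact and can be picked up again.
; BeginPlay applies a physics impulse along the player's facing, and Tick spins the axe in flight.
; Hitting a non-player freezes it with sound and effects, moving a pickup box there that restores HaveAxe and destroys the actor on player overlap.
; Recall interpolates axe and box toward the held axe, but nothing here runs it.
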(event `self.ReceiveHit`
  (params (MyComp :type "PrimitiveComponent Object Reference") (Other :type "Actor Object Reference") (OtherComp :type "PrimitiveComponent Object Reference") (bSelfMoved :type Boolean) (HitLocation :type "Vector Structure") (HitNormal :type "Vector Structure") (NormalImpulse :type "Vector Structure") (Hit :type "HitResult Structure (by ref)"))
  (bind (_bblockinghit _binitialoverlap _time _distance _location _impactpoint _normal _impactnormal _physmat _hitactor) (`GameplayStatics.BreakHitResult` Hit))
  (bind _a_simple_axx (`self.a_simple_axx`))
  (bind _asbp_third_person_character (cast `/Game/Blueprints/Characters/3rd_person_Blueprints/BP_ThirdPersonCharacter` (`GameplayStatics.GetPlayerPawn` 0)))
  (if (not (== _asbp_third_person_character Other))
    (`PrimitiveComponent.SetEnableGravity` (`self.a_simple_axx`) false)
    (`PrimitiveComponent.SetSimulatePhysics` (`self.a_simple_axx`) false)
    (`PrimitiveComponent.SetCollisionEnabled` _a_simple_axx "QueryOnly")
    (`SceneComponent.K2_SetWorldLocation` (`self.Box`) (`SceneComponent.K2_GetComponentLocation` _a_simple_axx) false false)
    (set `self.moveball` false)
    (`GameplayStatics.ApplyPointDamage` _hitactor 100.0 _impactnormal Hit (`GameplayStatics.GetPlayerController` 0) (`GameplayStatics.GetPlayerPawn` 0))
    (`GameplayStatics.PlaySoundAtLocation` "/Game/refereance/firstperson_bannasa/audio/shoot_sound.shoot_sound" (`self.K2_GetActorLocation`) (struct) 1.0 1.0 0.0 null null null null)
    (`NiagaraFunctionLibrary.SpawnSystemAtLocation` "/Game/ART/particles/FXS_ImpactBurst.FXS_ImpactBurst" _impactpoint)))

(event `self.ReceiveTick`
  (params (DeltaSeconds :type "Float (single-precision)"))
  (set `self.Delta Seconds` DeltaSeconds)
  (bind _asbp_third_person_character (cast `/Game/Blueprints/Characters/3rd_person_Blueprints/BP_ThirdPersonCharacter` (`GameplayStatics.GetPlayerPawn` 0)))
  (if (`/Game/Blueprints/Characters/3rd_person_Blueprints/BP_ThirdPersonCharacter.have axe` _asbp_third_person_character)
    _
    (elif (`self.moveball`)
      (`SceneComponent.K2_AddRelativeRotation` (`self.a_simple_axx`) (struct :`Roll` 20.0) true false))))

(event `self.ReceiveBeginPlay`
  (`SceneComponent.K2_SetWorldLocation` (`self.Box`) (0.0 0.0 1000.0) false true)
  (set `self.moveball` true)
  (`PrimitiveComponent.SetEnableGravity` (`self.a_simple_axx`) false)
  (`PrimitiveComponent.SetSimulatePhysics` (`self.a_simple_axx`) false)
  (bind _asbp_third_person_character (cast `/Game/Blueprints/Characters/3rd_person_Blueprints/BP_ThirdPersonCharacter` (`GameplayStatics.GetPlayerPawn` 0)))
  (bind _capsulecomponent (`Character.CapsuleComponent` _asbp_third_person_character))
  (`SceneComponent.K2_SetWorldLocation` (`self.a_simple_axx`) (`KismetMathLibrary.MakeVector` (.x (`SceneComponent.K2_GetComponentLocation` _capsulecomponent)) (.y (`SceneComponent.K2_GetComponentLocation` _capsulecomponent)) (+ (.z (`SceneComponent.K2_GetComponentLocation` _capsulecomponent)) 100.0)) false true)
  (`PrimitiveComponent.SetEnableGravity` (`self.a_simple_axx`) true)
  (`PrimitiveComponent.SetSimulatePhysics` (`self.a_simple_axx`) true)
  (`PrimitiveComponent.AddImpulse` (`self.a_simple_axx`) (`KismetMathLibrary.MakeVector` (.x (* (`KismetMathLibrary.GetForwardVector` (`SceneComponent.K2_GetComponentRotation` _capsulecomponent)) (`self.impulseMultiplier`))) (.y (* (`KismetMathLibrary.GetForwardVector` (`SceneComponent.K2_GetComponentRotation` _capsulecomponent)) (`self.impulseMultiplier`))) (+ (.z (* (`KismetMathLibrary.GetForwardVector` (`SceneComponent.K2_GetComponentRotation` _capsulecomponent)) (`self.impulseMultiplier`))) 3.0)) "None" false)
  (`SceneComponent.K2_SetWorldRotation` (`self.a_simple_axx`) (struct :`Pitch` 40.0 :`Roll` 300.0) true false))

(event `self.Box.OnComponentBeginOverlap`
  (params (OverlappedComponent :type "PrimitiveComponent Object Reference") (OtherActor :type "Actor Object Reference") (OtherComp :type "PrimitiveComponent Object Reference") (OtherBodyIndex :type Integer) (bFromSweep :type Boolean) (SweepResult :type "HitResult Structure (by ref)"))
  (bind _asbp_third_person_character (cast `/Game/Blueprints/Characters/3rd_person_Blueprints/BP_ThirdPersonCharacter` (`GameplayStatics.GetPlayerPawn` 0)))
  (if (== _asbp_third_person_character OtherActor)
    (bind _asbp_third_person_character_2 (cast `/Game/Blueprints/Characters/3rd_person_Blueprints/BP_ThirdPersonCharacter` (`GameplayStatics.GetPlayerPawn` 0)))
    (set `/Game/Blueprints/Characters/3rd_person_Blueprints/BP_ThirdPersonCharacter.have axe` true _asbp_third_person_character_2)
    (`self.K2_DestroyActor`)))

(fn `location control`
  (params (`position of character ` :type "Vector Structure") (`end location` :type "Vector Structure"))
  (locals (NewLocalVar :type "SceneComponent Object Reference")))

(fn `Recall`
  (params (`elapsed time` :type "Float (double-precision)"))
  (bind _a_simple_axx (`self.a_simple_axx`))
  (set `self.Elapsed Time` `elapsed time`)
  (bind _asbp_third_person_character (cast `/Game/Blueprints/Characters/3rd_person_Blueprints/BP_ThirdPersonCharacter` (`GameplayStatics.GetPlayerPawn` 0)))
  (set `self.axe in hand current location` (`SceneComponent.K2_GetComponentLocation` (`/Game/Blueprints/Characters/3rd_person_Blueprints/BP_ThirdPersonCharacter.BP_axe` _asbp_third_person_character)))
  (set `self.Floating return axe Curennt location` (`SceneComponent.K2_GetComponentLocation` (`self.a_simple_axx`)))
  (set `self.interp speed` (`KismetMathLibrary.SafeDivide` (`KismetMathLibrary.Vector_Distance` (`self.Floating return axe Curennt location`) (`self.axe in hand current location`)) 150.0))
  (set `self.moving rotaion` (`KismetMathLibrary.Conv_VectorToRotator` (`KismetMathLibrary.VInterpTo` (`KismetMathLibrary.Conv_RotatorToVector` (`SceneComponent.K2_GetComponentRotation` (`self.a_simple_axx`))) (`KismetMathLibrary.Conv_RotatorToVector` (`SceneComponent.K2_GetComponentRotation` (`/Game/Blueprints/Characters/3rd_person_Blueprints/BP_ThirdPersonCharacter.BP_axe` _asbp_third_person_character))) (`self.Elapsed Time`) (`self.interp speed`))))
  (set `self.new Location of floating axe` (`KismetMathLibrary.VInterpTo` (`self.Floating return axe Curennt location`) (`self.axe in hand current location`) (`self.Elapsed Time`) (`self.interp speed`)))
  (`SceneComponent.K2_SetWorldLocation` (`self.a_simple_axx`) (`self.new Location of floating axe`) false false)
  (`SceneComponent.K2_SetWorldLocation` (`self.Box`) (`self.new Location of floating axe`) false false)
  (`/Engine/EditorBlueprintResources/StandardMacros.IsValid` _a_simple_axx
    (:`Is Valid`
      (`SceneComponent.K2_SetWorldRotation` _a_simple_axx (`self.moving rotaion`) false false)
      (`SceneComponent.K2_SetWorldRotation` (`self.Box`) (`self.moving rotaion`) false false))))

(fn `testMoveBall`)

(fn `UserConstructionScript`)