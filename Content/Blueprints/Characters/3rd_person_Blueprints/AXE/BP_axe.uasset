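; BP_axe is a melee axe that deals point damage to actors its Box collision overlaps, excluding the player's BP_ThirdPersonCharacter.
; Each tick it copies the player's AxeInUseCanDealDamage flag to switch the Box between query-only and no collision.
; A failed cast on tick also enables the Box.
; Damage uses the player's forward vector, the Box location in a constructed hit result, and the player as causer.
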(event `self.Box.OnComponentBeginOverlap`
  (params (OverlappedComponent :type "PrimitiveComponent Object Reference") (OtherActor :type "Actor Object Reference") (OtherComp :type "PrimitiveComponent Object Reference") (OtherBodyIndex :type Integer) (bFromSweep :type Boolean) (SweepResult :type "HitResult Structure (by ref)"))
  (bind _returnvalue (`SceneComponent.K2_GetComponentLocation` (`self.Box`)))
  (bind _asbp_third_person_character (cast `/Game/Blueprints/Characters/3rd_person_Blueprints/BP_ThirdPersonCharacter` (`GameplayStatics.GetPlayerPawn` 0)))
  (if (not (== _asbp_third_person_character OtherActor))
    (bind _asbp_third_person_character_2 (cast `/Game/Blueprints/Characters/3rd_person_Blueprints/BP_ThirdPersonCharacter` (`GameplayStatics.GetPlayerPawn` 0)))
    (`GameplayStatics.ApplyPointDamage` OtherActor (`self.Amount of damge axe deals`) (`self.GetActorForwardVector` _asbp_third_person_character_2) (`GameplayStatics.MakeHitResult` false true 0.0 0.0 _returnvalue _returnvalue (0.0 0.0 1.0) (0.0 0.0 1.0) null OtherActor) null _asbp_third_person_character_2)))

(event `self.ReceiveTick`
  (params (DeltaSeconds :type "Float (single-precision)"))
  (bind _asbp_third_person_character (cast `/Game/Blueprints/Characters/3rd_person_Blueprints/BP_ThirdPersonCharacter` (`GameplayStatics.GetPlayerPawn` 0))
    (:`then`
      (bind _output_get (set `self.should_axe_deal_damage` (`/Game/Blueprints/Characters/3rd_person_Blueprints/BP_ThirdPersonCharacter.axe_in_use_can_deal_damage` _asbp_third_person_character)))
      (if _output_get
        (`PrimitiveComponent.SetCollisionEnabled` (`self.Box`) "QueryOnly" :!label _label)
        (else
          (`PrimitiveComponent.SetCollisionEnabled` (`self.Box`) "NoCollision"))))
    (:`CastFailed`
      (goto _label))))

(fn `UserConstructionScript`)