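; Slime enemy that is marked dead when the player's character overlaps its sphere, with its alive state kept across level loads.
; The state lives in the SlimesAlive map on the BP_level_information_store game instance, keyed by actor display name.
; BeginPlay registers unknown slimes as alive and restores the dead look for known dead ones.
; Death only updates the map and swaps the mesh material; the actor is not destroyed.
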(event `self.ReceiveBeginPlay`
  (`self.on level entry detect status`))

(event `self.Sphere.OnComponentBeginOverlap`
  (params (OverlappedComponent :type "PrimitiveComponent Object Reference") (OtherActor :type "Actor Object Reference") (OtherComp :type "PrimitiveComponent Object Reference") (OtherBodyIndex :type Integer) (bFromSweep :type Boolean) (SweepResult :type "HitResult Structure (by ref)"))
  (bind _returnvalue (`KismetStringLibrary.Conv_StringToName` (`KismetSystemLibrary.GetDisplayName` self)))
  ; on death
  (bind _asbp_third_person_character (cast `/Game/Blueprints/Characters/3rd_person_Blueprints/BP_ThirdPersonCharacter` (`GameplayStatics.GetPlayerPawn` 0)))
  (if (== _asbp_third_person_character OtherActor)
    (bind _asbp_level_information_store (cast `/Game/Blueprints/BP_level_information_store` (`GameplayStatics.GetGameInstance`)))
    (bind _slimes__alive (`/Game/Blueprints/BP_level_information_store.slimes_ alive` _asbp_level_information_store))
    (`BlueprintMapLibrary.Map_Remove` _slimes__alive _returnvalue)
    (`BlueprintMapLibrary.Map_Add` _slimes__alive _returnvalue) ; if slime display name not here add it and set is alive boolen to true
    (`PrimitiveComponent.SetMaterial` (`self.slime mesh`) 0 "/Engine/MapTemplates/Materials/BasicAsset01.BasicAsset01")))

(fn `on level entry detect status`
  ; on level entry check with game instancer if is in the map of known living slimes, if no add, if yes change material if dead
  (bind _asbp_level_information_store (cast `/Game/Blueprints/BP_level_information_store` (`GameplayStatics.GetGameInstance`)))
  (bind (_value _returnvalue) (`BlueprintMapLibrary.Map_Find` (`/Game/Blueprints/BP_level_information_store.slimes_ alive` _asbp_level_information_store) (`KismetStringLibrary.Conv_StringToName` (`KismetSystemLibrary.GetDisplayName` self))))
  (if _returnvalue
    (if (not _value)
      (`PrimitiveComponent.SetMaterial` (`self.slime mesh`) 0 "/Engine/MapTemplates/Materials/BasicAsset01.BasicAsset01"))
    (else
      (bind _asbp_level_information_store_2 (cast `/Game/Blueprints/BP_level_information_store` (`GameplayStatics.GetGameInstance`)))
      (`BlueprintMapLibrary.Map_Add` (`/Game/Blueprints/BP_level_information_store.slimes_ alive` _asbp_level_information_store_2) (`KismetStringLibrary.Conv_StringToName` (`KismetSystemLibrary.GetDisplayName` self)) true) ; if slime display name not here add it and set is alive boolen to true
    )))

(fn `UserConstructionScript`)