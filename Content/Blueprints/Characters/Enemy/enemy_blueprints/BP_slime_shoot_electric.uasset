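; Electric slime enemy that patrols random navmesh points, idles between patrols and attacks the player with a lightning ball.
; Tick drives a boolean state machine: pawn sensing triggers charging and a retreat if too close, then it fires once the scaling ball reaches full size.
; It saves position and alive state by display name in the game instance to restore on level entry.
; At zero health it spawns a collectable.
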(event `self.ReceiveBeginPlay`
  (`SceneComponent.SetVisibility` (`self.BP_newball`) true false)
  (set `/Game/Blueprints/Components/BP_healthSystemComponent.maxHealth` 10.0 (`self.BP_healthSystemComponent`))
  ; on level entry check with game instancer if information about self is stored and act acordingly
  (set `/Game/Blueprints/Components/BP_trapcountdown.timeleft` 10.0 (`self.BP_trapcountdown`))
  (`self.Update_My_information` false))

(event `self.PawnSensing.OnSeePawn`
  (params (Pawn :type "Pawn Object Reference"))
  (bind _returnvalue (`GameplayStatics.GetPlayerPawn` 0))
  (bind _asbp_third_person_character (cast `/Game/Blueprints/Characters/3rd_person_Blueprints/BP_ThirdPersonCharacter` _returnvalue))
  (if (== Pawn _returnvalue)
    (bind (_projectedlocation _returnvalue_2) (`NavigationSystemV1.K2_ProjectPointToNavigation` (`self.K2_GetActorLocation` _asbp_third_person_character) (`self.nav data`)))
    (set `self.player seen location` _projectedlocation)
    (if _returnvalue_2
      (set `self.see Charater` true))))

(event `self.OnLanded`
  (params (Hit :type "HitResult Structure (by ref)"))
  ; attack on landed from jump
  (`PrimitiveComponent.SetMaterial` (`self.Mesh`) 0 "/Engine/EngineMaterials/EmissiveTexturedMaterial.EmissiveTexturedMaterial"))

(event `self.ReceiveTick`
  (params (DeltaSeconds :type "Float (single-precision)"))
  (bind _bp_trapcountdown (`self.BP_trapcountdown`))
  (bind _charactermovement (`self.CharacterMovement`))
  (bind _how_many_patrols_before_idel (`self.how many patrols before idel`))
  (bind _bp_trapcountdown_2 (`self.BP_trapcountdown`))
  (bind _returnvalue (`AIBlueprintHelperLibrary.GetAIController` self))
  (bind _timeleft (`/Game/Blueprints/Components/BP_trapcountdown.timeleft` _bp_trapcountdown))
  (bind _timeleft_2 (`/Game/Blueprints/Components/BP_trapcountdown.timeleft` _bp_trapcountdown_2))
  (bind (_randomlocation _returnvalue_2) (`NavigationSystemV1.K2_GetRandomReachablePointInRadius` (`self.GetNavAgentLocation` self) (`self.search raduis`) (`self.nav data`) null))
  (if (== 0.0 (`/Game/Blueprints/Components/BP_healthSystemComponent.health` (`self.BP_healthSystemComponent`)))
    (`self.remove me from living map add to dead`)
    (`|SpawnActorFromClass` "/Game/Blueprints/BP_collectable.BP_collectable_C" (`self.GetTransform`) "Undefined" "MultiplyWithRoot" null null)
    (else
      (`self.Update_My_information` true)
      (if (`self.see Charater`)
        (`self.Charge up attack`)
        (if (`self.first tiem charater seen`)
          (set `self.attacking` true)
          (set `self.first tiem charater seen` false)
          (if (<= (`KismetMathLibrary.Vector_Distance` (`self.K2_GetActorLocation`) (`self.player seen location`)) (`self.stop run and attack range `))
            (set `CharacterMovementComponent.MaxWalkSpeed` 300.0 (`self.CharacterMovement`))
            (`self.calc run away location`)
            (`|AIMoveTo` (`self.CharacterMovement`) self (`self.runaway location`) null (`self.accepted stoping radius`) true
              (:`OnSuccess`
                _)))
          (bind _asbp_third_person_character (cast `/Game/Blueprints/Characters/3rd_person_Blueprints/BP_ThirdPersonCharacter` (`GameplayStatics.GetPlayerPawn` 0)))
          (`AIController.K2_SetFocus` _returnvalue _asbp_third_person_character)
          (`KismetSystemLibrary.Delay` 0.1)
          (`AIController.K2_ClearFocus` _returnvalue)
          (set `self.see Charater` false)
          (set `self.first tiem charater seen` true)
          (set `self.patrolling` true)
          (set `self.need location for patrol ` true))
        (elif (`self.attacking`)
          (if (`self.fully charged ball`)
            (bind _asbp_third_person_character_2 (cast `/Game/Blueprints/Characters/3rd_person_Blueprints/BP_ThirdPersonCharacter` (`GameplayStatics.GetPlayerPawn` 0)))
            (`AIController.K2_SetFocus` (`AIBlueprintHelperLibrary.GetAIController` self) _asbp_third_person_character_2)
            (if (`self.attack 1`)
              (`self.ATTACK`))
            (else
              (`self.Charge up attack`)))
          (elif (`self.idel`)
            (`/Game/Blueprints/Components/BP_trapcountdown.countdown` _bp_trapcountdown _timeleft 0.0 0.0)
            (if (== _timeleft 0.0)
              (set `self.idel` false)
              (set `self.first idel` true)
              (set `self.patrolling` true)
              (set `self.need location for patrol ` true))
            (elif (`self.patrolling`)
              (if (`self.need location for patrol `)
                (set `self.need location for patrol ` false)
                (if _returnvalue_2
                  (set `self.patrol location` _randomlocation)
                  (set `self.patrol location ready` true)
                  (set `/Game/Blueprints/Components/BP_trapcountdown.timeleftbig` _how_many_patrols_before_idel (`self.BP_trapcountdown`))
                  (set `self.active patrol` true)
                  (if (== 0.0 _how_many_patrols_before_idel)
                    (set `self.idel` true)
                    (set `/Game/Blueprints/Components/BP_trapcountdown.timeleft` 100.0 (`self.BP_trapcountdown`))))
                (elif (`self.patroltimercountdown`)
                  (`/Game/Blueprints/Components/BP_trapcountdown.countdown` _bp_trapcountdown_2 _timeleft_2 0.0 0.0)
                  (if (== _timeleft_2 0.0)
                    (set `self.need location for patrol ` true)
                    (set `self.patroltimercountdown` false)
                    (set `/Game/Blueprints/Components/BP_trapcountdown.timeleft` (`self.patrol cooldown`) (`self.BP_trapcountdown`)))
                  (elif (`self.active patrol`)
                    (set `self.active patrol` false)
                    (set `CharacterMovementComponent.MaxWalkSpeed` 150.0 _charactermovement)
                    (`|AIMoveTo` _charactermovement self (`self.patrol location`) null (`self.accepted stoping radius`) true
                      (:`OnSuccess`
                        (set `self.patroltimercountdown` true)))))))))))))

(fn `ATTACK`
  (set `self.attack 1` false)
  (`SceneComponent.SetVisibility` (`self.BP_newball`) true false)
  (`|SpawnActorFromClass` "/Game/ART/particles/Partical_Materials/Lightning/BP_LightningBall_throw.BP_LightningBall_throw_C" (`KismetMathLibrary.MakeTransform` (+ (`self.K2_GetActorLocation`) (50.0 0.0 0.0)) (struct) (0.1 0.1 0.1)) "AdjustIfPossibleButAlwaysSpawn" "MultiplyWithRoot" null self)
  (set `self.attacking` false))

(fn `calc run away location`
  (bind _returnvalue (`self.K2_GetActorLocation`))
  (bind _player_seen_location (`self.player seen location`))
  (set `self.runaway location` (`NavigationSystemV1.K2_ProjectPointToNavigation` (+ (* (`KismetMathLibrary.Normal` (- _returnvalue _player_seen_location)) (- (`self.stop run and attack range `) (`KismetMathLibrary.Vector_Distance` _returnvalue _player_seen_location))) (`self.K2_GetActorLocation`)) (`self.nav data`))))

(fn `Charge up attack`
  (bind _returnvalue (`KismetMathLibrary.FClamp` (+ (`self.current charge up size`) 0.01)))
  (if (`self.first charge`)
    (`SceneComponent.SetVisibility` (`self.BP_newball`) true false)
    (set `self.first charge` false)
    (elif (`self.charging`)
      (`SceneComponent.SetRelativeScale3D` (`self.BP_newball`) (`KismetMathLibrary.Conv_DoubleToVector` _returnvalue))
      (set `self.current charge up size` _returnvalue)
      (if (== (`self.current charge up size`) 1.0)
        (set `self.fully charged ball` true)
        (set `self.charging` false)
        (set `self.first charge` true)))))

(fn `is in view`)

(fn `Level_information_storeage_reader`
  (returns (already_exists_alive :type Boolean) (alive :type Boolean) (already_exists_start_location :type Boolean) (start_location :type "Vector Structure") (already_exists_current_location :type Boolean) (current_location :type "Vector Structure"))
  (bind _asbp_level_information_store (cast `/Game/Blueprints/BP_level_information_store` (`GameplayStatics.GetGameInstance`)))
  (bind (_value _returnvalue) (`BlueprintMapLibrary.Map_Find` (`/Game/Blueprints/BP_level_information_store.slimes_ alive` _asbp_level_information_store) (`self.My_Displayname`)))
  (bind (_value_2 _returnvalue_2) (`BlueprintMapLibrary.Map_Find` (`/Game/Blueprints/BP_level_information_store.slime_starting_location` _asbp_level_information_store) (`self.My_Displayname`)))
  (bind (_value_3 _returnvalue_3) (`BlueprintMapLibrary.Map_Find` (`/Game/Blueprints/BP_level_information_store.slime_current_location` _asbp_level_information_store) (`self.My_Displayname`)))
  (return _returnvalue _value _returnvalue_2 _value_2 _returnvalue_3 _value_3))

(fn `remove me from living map add to dead`
  (bind _returnvalue (`KismetStringLibrary.Conv_StringToName` (`KismetSystemLibrary.GetDisplayName` self)))
  (bind _asbp_level_information_store (cast `/Game/Blueprints/BP_level_information_store` (`GameplayStatics.GetGameInstance`)))
  (bind _slimes__alive (`/Game/Blueprints/BP_level_information_store.slimes_ alive` _asbp_level_information_store))
  (`BlueprintMapLibrary.Map_Remove` _slimes__alive _returnvalue)
  (`BlueprintMapLibrary.Map_Add` _slimes__alive _returnvalue true) ; if slime display name not here add it and set is alive boolen to true
  (`self.K2_DestroyActor`))

(fn `Update_My_information`
  (params (`update only current location` :type Boolean))
  (if `update only current location`
    (bind _asbp_level_information_store (cast `/Game/Blueprints/BP_level_information_store` (`GameplayStatics.GetGameInstance`)))
    (`BlueprintMapLibrary.Map_Add` (`/Game/Blueprints/BP_level_information_store.slime_current_location` _asbp_level_information_store) (`self.My_Displayname`) (`self.K2_GetActorLocation`))
    (else
      (bind _asbp_level_information_store_2 (cast `/Game/Blueprints/BP_level_information_store` (`GameplayStatics.GetGameInstance`)))
      (bind (_already_exists_alive _alive _already_exists_start_location _start_location _already_exists_current_location _current_location) (`self.Level_information_storeage_reader`))
      (if (not _already_exists_alive)
        (`BlueprintMapLibrary.Map_Add` (`/Game/Blueprints/BP_level_information_store.slimes_ alive` _asbp_level_information_store_2) (`self.My_Displayname`) true))
      (if (`BlueprintMapLibrary.Map_Find` (`/Game/Blueprints/BP_level_information_store.slimes_ alive` _asbp_level_information_store_2) (`self.My_Displayname`))
        (if (not _already_exists_start_location)
          (`BlueprintMapLibrary.Map_Add` (`/Game/Blueprints/BP_level_information_store.slime_starting_location` _asbp_level_information_store_2) (`self.My_Displayname`) (`self.K2_GetActorLocation`)))
        (if _already_exists_current_location
          (`self.K2_SetActorLocation` _current_location false true))
        (else
          ; already dead
          (`self.K2_DestroyActor`))))))

(fn `UserConstructionScript`)