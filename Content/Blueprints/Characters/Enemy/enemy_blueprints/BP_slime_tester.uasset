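; Slime enemy character that patrols the navmesh and chases the player's last seen location, spawning a collectable when its health reaches zero.
; BeginPlay records it by display name in the game instance's SlimesAlive map, or destroys it if already marked dead there.
; Tick runs a flag-based state machine using PawnSensing, AIMoveTo and countdown-component timers.
; Chasing is never cleared in live logic, so patrol stops after a first sighting.
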(event `self.ReceiveBeginPlay`
  (set `/Game/Blueprints/Components/BP_healthSystemComponent.maxHealth` 10.0 (`self.BP_healthSystemComponent`))
  ; on level entry check with game instancer if is in the map of known living slimes, if no add, if yes change material if dead
  (set `/Game/Blueprints/Components/BP_trapcountdown.timeleft` 10.0 (`self.BP_trapcountdown`))
  (bind _asbp_level_information_store (cast `/Game/Blueprints/BP_level_information_store` (`GameplayStatics.GetGameInstance`)))
  (bind (_value _returnvalue) (`BlueprintMapLibrary.Map_Find` (`/Game/Blueprints/BP_level_information_store.slimes_ alive` _asbp_level_information_store) (`KismetStringLibrary.Conv_StringToName` (`KismetSystemLibrary.GetDisplayName` self))))
  (if _returnvalue
    (if (not _value)
      (`self.K2_DestroyActor`))
    (else
      (bind _asbp_level_information_store_2 (cast `/Game/Blueprints/BP_level_information_store` (`GameplayStatics.GetGameInstance`)))
      (`BlueprintMapLibrary.Map_Add` (`/Game/Blueprints/BP_level_information_store.slimes_ alive` _asbp_level_information_store_2) (`KismetStringLibrary.Conv_StringToName` (`KismetSystemLibrary.GetDisplayName` self)) true) ; if slime display name not here add it and set is alive boolen to true
    )))

(event `self.PawnSensing.OnSeePawn`
  (params (Pawn :type "Pawn Object Reference"))
  (bind _returnvalue (`GameplayStatics.GetPlayerPawn` 0))
  (bind _asbp_third_person_character (cast `/Game/Blueprints/Characters/3rd_person_Blueprints/BP_ThirdPersonCharacter` _returnvalue))
  (if (== Pawn _returnvalue)
    (bind (_projectedlocation _returnvalue_2) (`NavigationSystemV1.K2_ProjectPointToNavigation` (`self.K2_GetActorLocation` _asbp_third_person_character) (`self.nav data`)))
    (set `self.player seen location` _projectedlocation)
    (if _returnvalue_2
      (set `self.see Charater` true))))

(event `self.ReceiveTick`
  (params (DeltaSeconds :type "Float (single-precision)"))
  (bind _bp_trapcountdown (`self.BP_trapcountdown`))
  (bind _charactermovement (`self.CharacterMovement`))
  (bind _how_many_patrols_before_idel (`self.how many patrols before idel`))
  (bind _bp_trapcountdown_2 (`self.BP_trapcountdown`))
  (bind _timeleft (`/Game/Blueprints/Components/BP_trapcountdown.timeleft` _bp_trapcountdown))
  (bind _timeleft_2 (`/Game/Blueprints/Components/BP_trapcountdown.timeleft` _bp_trapcountdown_2))
  (bind (_randomlocation _returnvalue) (`NavigationSystemV1.K2_GetRandomReachablePointInRadius` (`self.GetNavAgentLocation` self) (`self.search raduis`) (`self.nav data`) null))
  (if (== 0.0 (`/Game/Blueprints/Components/BP_healthSystemComponent.health` (`self.BP_healthSystemComponent`)))
    (`self.remove me from living map add to dead`)
    (`|SpawnActorFromClass` "/Game/Blueprints/BP_collectable.BP_collectable_C" (`self.GetTransform`) "Undefined" "MultiplyWithRoot" null null)
    (elif (`self.see Charater`)
      (if (`self.first tiem charater seen`)
        (set `self.chasing` true)
        (set `self.first tiem charater seen` false)
        (set `CharacterMovementComponent.MaxWalkSpeed` 300.0 (`self.CharacterMovement`))
        (`|AIMoveTo` (`self.CharacterMovement`) self (`self.player seen location`) null (`self.accepted stoping radius`) true
          (:`OnSuccess`
            (set `self.see Charater` false)
            (set `self.first tiem charater seen` true)
            (set `self.patrolling` true)
            (set `self.need location for patrol ` true))))
      (elif (`self.chasing`)
        _
        (elif (`self.idel`)
          (`/Game/Blueprints/Components/BP_trapcountdown.countdown` _bp_trapcountdown _timeleft 0.0 0.0)
          (if (== _timeleft 0.0)
            (set `self.idel` false)
            (set `self.first idel` true)
            (set `self.patrolling` true)
            (set `self.need location for patrol ` true))
          (elif (`self.patrolling`)
            (if (`self.need location for patrol `)
              (set `self.need location for patrol ` false)
              (if _returnvalue
                (set `self.patrol location` _randomlocation)
                (set `self.patrol location ready` true)
                (set `/Game/Blueprints/Components/BP_trapcountdown.timeleftbig` _how_many_patrols_before_idel (`self.BP_trapcountdown`))
                (set `self.active patrol` true)
                (if (== 0.0 _how_many_patrols_before_idel)
                  (set `self.idel` true)
                  (set `/Game/Blueprints/Components/BP_trapcountdown.timeleft` 100.0 (`self.BP_trapcountdown`))))
              (elif (`self.patroltimercountdown`)
                (`/Game/Blueprints/Components/BP_trapcountdown.countdown` _bp_trapcountdown_2 _timeleft_2 0.0 0.0)
                (if (== _timeleft_2 0.0)
                  (set `self.need location for patrol ` true)
                  (set `self.patroltimercountdown` false)
                  (set `/Game/Blueprints/Components/BP_trapcountdown.timeleft` (`self.patrol cooldown`) (`self.BP_trapcountdown`)))
                (elif (`self.active patrol`)
                  (set `self.active patrol` false)
                  (set `CharacterMovementComponent.MaxWalkSpeed` 150.0 _charactermovement)
                  (`|AIMoveTo` _charactermovement self (`self.patrol location`) null (`self.accepted stoping radius`) true
                    (:`OnSuccess`
                      (set `self.patroltimercountdown` true))))))))))))

(fn `is in view`)

(fn `NewFunction`)

(fn `remove me from living map add to dead`
  (bind _returnvalue (`KismetStringLibrary.Conv_StringToName` (`KismetSystemLibrary.GetDisplayName` self)))
  (bind _asbp_level_information_store (cast `/Game/Blueprints/BP_level_information_store` (`GameplayStatics.GetGameInstance`)))
  (bind _slimes__alive (`/Game/Blueprints/BP_level_information_store.slimes_ alive` _asbp_level_information_store))
  (`BlueprintMapLibrary.Map_Remove` _slimes__alive _returnvalue)
  (`BlueprintMapLibrary.Map_Add` _slimes__alive _returnvalue) ; if slime display name not here add it and set is alive boolen to true
  (`self.K2_DestroyActor`))

(fn `UserConstructionScript`)