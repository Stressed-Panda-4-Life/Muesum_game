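; Interactable lava actor whose StartInteract event currently only prints a "fight me" debug string.
; Disconnected logic would toggle four Niagara effects with the player character's SideWaysPlatformMoving flag, using MoveSwitch and StopSwitch so each change fires once.
; A second disconnected chain would set Interacting and flag PlatformInteract on the player character.
; Tick is empty, so neither chain runs.
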(event `/Game/Blueprints/Input/BPI_interact.start interact`
  (`KismetSystemLibrary.PrintString` "fight me"))

(event `self.ReceiveTick`
  (params (DeltaSeconds :type "Float (single-precision)")))

(fn `UserConstructionScript`
  (`parent.UserConstructionScript`))