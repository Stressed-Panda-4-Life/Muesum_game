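; Interactable platform actor meant to move a child actor between a low and a high point when the player is inside its box.
; StartInteract checks player overlap, waits, then flips direction and sets the target, moving flag and a per-direction speed.
; The interpolated movement, sound and character-flag logic is disconnected and Tick is empty, so nothing in this graph currently moves the platform.
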(event `self.ReceiveBeginPlay`
  (set `self.target` (`SceneComponent.K2_GetComponentLocation` (`self.low point`)))
  (set `self.Platform` (`SceneComponent.K2_GetComponentLocation` (`self.ChildActor`))))

(event `self.Box.OnComponentBeginOverlap`
  (params (OverlappedComponent :type "PrimitiveComponent Object Reference") (OtherActor :type "Actor Object Reference") (OtherComp :type "PrimitiveComponent Object Reference") (OtherBodyIndex :type Integer) (bFromSweep :type Boolean) (SweepResult :type "HitResult Structure (by ref)"))
  (if (== OtherActor (`GameplayStatics.GetPlayerPawn` 0))
    (set `self.detect player` true)))

(event `self.Box.OnComponentEndOverlap`
  (params (OverlappedComponent :type "PrimitiveComponent Object Reference") (OtherActor :type "Actor Object Reference") (OtherComp :type "PrimitiveComponent Object Reference") (OtherBodyIndex :type Integer))
  (if (== OtherActor (`GameplayStatics.GetPlayerPawn` 0))
    (set `self.detect player` false)))

(event `self.ReceiveTick`
  (params (DeltaSeconds :type "Float (single-precision)")))

(event `/Game/Blueprints/Input/BPI_interact.start interact`
  (`KismetSystemLibrary.PrintString` "Hello")
  (if (`self.detect player`)
    (if (`self.going down`)
      (`KismetSystemLibrary.Delay` 1.0)
      (set `self.going down` false)
      (set `self.target` (`SceneComponent.K2_GetComponentLocation` (`self.highpoint`)))
      (set `self.moving` true)
      (set `self.Interp Speed` 100.0)
      (else
        (`KismetSystemLibrary.Delay` 4.0)
        (set `self.going down` true)
        (set `self.target` (`SceneComponent.K2_GetComponentLocation` (`self.low point`)))
        (set `self.moving` true)
        (set `self.Interp Speed` 400.0)))))

(fn `get position`)

(fn `UserConstructionScript`
  (`parent.UserConstructionScript`))