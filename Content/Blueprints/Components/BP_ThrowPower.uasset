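; BP_ThrowPower is a component managing a regenerating throw-power meter, apparently for the first-person character's bomb throw.
; If the character's Bombthrownow is set at BeginPlay, power starts at minimum and a looping timer regenerates it, clamped to maximum and printed.
; Stamina-named functions pause, resume or spend power.
; Spending pauses regeneration and sets a looping resume timer, using the configured pause duration when power is low, otherwise a fixed delay.
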(event `self.ReceiveBeginPlay`
  (bind _asbp_first_person_character (cast `/Game/refereance/firstperson_bannasa/Blueprints/BP_FirstPersonCharacter` (`GameplayStatics.GetPlayerPawn` 0)))
  (if (`/Game/refereance/firstperson_bannasa/Blueprints/BP_FirstPersonCharacter.bombthrownow` _asbp_first_person_character)
    (set `self.throwPower` (`self.minimum_throwPower`))
    (bind _returnvalue (`KismetSystemLibrary.K2_SetTimer` null "Tick throw_power" (`self.powerTickFrequency`) true))
    (set `self.throwPowerTickTimer` _returnvalue)))

(fn `pauseTickStamina`
  (params (duration :type "Float (double-precision)"))
  (`KismetSystemLibrary.K2_PauseTimerHandle` (`self.throwPowerTickTimer`))
  (if (> 2.0 (`self.throwPower`))
    (`KismetSystemLibrary.K2_SetTimer` null "StartTickStamina" (`self.ThrowPowerPauseDuration`) true)
    (else
      (`KismetSystemLibrary.K2_SetTimer` null "StartTickStamina" 1.0 true))))

(fn `spendStamina`
  (params (amount :type "Float (double-precision)"))
  (if (> amount 0.0)
    (set `self.throwPower` (`KismetMathLibrary.FClamp` (- (`self.throwPower`) amount) 0.0 (`self.MaxThrowPower`)))
    (`self.pauseTickStamina` (`self.ThrowPowerPauseDuration`))))

(fn `StartTickStamina`
  (`KismetSystemLibrary.K2_UnPauseTimerHandle` (`self.throwPowerTickTimer`)))

(fn `stopTickStamina`
  (`KismetSystemLibrary.K2_PauseTimerHandle` (`self.throwPowerTickTimer`)))

(fn `Tick throw_power`
  (bind _output_get (set `self.throwPower` (`KismetMathLibrary.FClamp` (+ (`self.throwPower`) (* (`self.ThrowPowerRegenPerSec`) (`self.powerTickFrequency`))) 0.0 (`self.MaxThrowPower`))))
  (`KismetSystemLibrary.PrintString` (`KismetStringLibrary.Conv_DoubleToString` _output_get)))