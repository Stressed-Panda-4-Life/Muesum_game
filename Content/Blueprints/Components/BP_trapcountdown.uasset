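; Trap countdown component, by its name, that lowers clamped time-left values in half-second steps.
; BeginPlay starts a looping timer targeting Countdown by name, although that function takes inputs, which such timers do not support.
; NewFunction pauses and re-sets the timer according to time left, and Countdownbig mirrors Countdown for a second value, but neither is called here.
; Player walk-speed and speed-boost reset logic is disconnected and never runs.
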(event `CustomEvent`)

(event `self.ReceiveBeginPlay`
  (bind _returnvalue (`KismetSystemLibrary.K2_SetTimer` null "countdown" (`self.tick freq`) true))
  (set `self.NewVar` _returnvalue))

(event `self.ReceiveTick`
  (params (DeltaSeconds :type "Float (single-precision)")))

(fn `countdown`
  (params (`applied time` :type "Float (double-precision)") (`change varible` :type "Float (double-precision) (by ref)") (`reset value` :type "Float (double-precision)"))
  (set `self.timeleft` (`KismetMathLibrary.FClamp` (- `applied time` 0.5) 0.0 30.0)))

(fn `countdownbig`
  (params (`applied time` :type "Float (double-precision)") (`change varible` :type "Float (double-precision) (by ref)") (`reset value` :type "Float (double-precision)"))
  (set `self.timeleftbig` (`KismetMathLibrary.FClamp` (- `applied time` 0.5) 0.0 30.0)))

(fn `NewFunction`
  (`KismetSystemLibrary.K2_PauseTimerHandle` (`self.NewVar`))
  (if (> 2.0 (`self.timeleft`))
    (`KismetSystemLibrary.K2_SetTimer` null "countdown" 0.0 true)
    (else
      (`KismetSystemLibrary.K2_SetTimer` null "countdown" 1.0 true))))