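; Actor component that provides a sprint ability by switching a character's maximum walk speed.
; StartSprint and StopSprint each take a character movement reference, check IsSprinting, then apply SprintSpeed or WalkSpeed.
; StopSprint sets IsSprinting to true instead of clearing it, so StartSprint has no effect after the first sprint.
; The event graph holds only disabled placeholder events, so both functions rely on external callers.
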(fn `startSprint`
  (params (`character movment` :type "CharacterMovementComponent Object Reference"))
  (if (not (`self.isSprinting`))
    (set `self.isSprinting` true)
    (set `CharacterMovementComponent.MaxWalkSpeed` (`self.SprintSpeed`) `character movment`)))

(fn `stopSprint`
  (params (`character movemnt` :type "CharacterMovementComponent Object Reference"))
  (if (`self.isSprinting`)
    (set `self.isSprinting` true)
    (set `CharacterMovementComponent.MaxWalkSpeed` (`self.walkSpeed`) `character movemnt`)))