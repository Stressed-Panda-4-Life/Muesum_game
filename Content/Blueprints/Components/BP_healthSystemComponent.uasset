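; Health component that tracks its owning actor's health, handling damage, healing and death.
; On BeginPlay it fills health and binds to the owner's OnTakeAnyDamage, then clamps each hit, plays sound and particle effects and fires OnTookDamage, plus OnKill at zero.
; Heal adds clamped health with its own effects and sets a Healing flag that never resets.
; Screenshake is set on every hit but cleared only after death; Kill and TakeDamage are empty.
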(event `self.ReceiveBeginPlay`
  (set `self.owner` (`self.GetOwner`))
  (set `self.health` (`self.maxHealth`))
  (add `Actor.OnTakeAnyDamage` (`self.owner`) (`|CreateDelegate` :!event `TookDamage`)))

(event `TookDamage`
  (params (DamagedActor :type "Actor Object Reference") (Damage :type "Float (single-precision)") (DamageType :type "DamageType Object Reference") (InstigatedBy :type "Controller Object Reference") (DamageCauser :type "Actor Object Reference"))
  (set `self.screenshake` true)
  (set `self.health` (`KismetMathLibrary.FClamp` (- (`self.health`) Damage) 0.0 (`self.maxHealth`)))
  (`self.playFX`)
  (`self.onTookDamage` Damage)
  (`KismetSystemLibrary.PrintString` (`KismetStringLibrary.Conv_DoubleToString` (`self.health`)))
  (if (<= (`self.health`) 0.0)
    (`self.onKill`)
    (`KismetSystemLibrary.Delay` 0.2)
    (set `self.screenshake` false)))

(fn `heal`
  (params (amount :type "Float (double-precision)"))
  (bind _returnvalue (`Actor.K2_GetActorLocation` (`self.owner`)))
  (bind _output_get (set `self.health` (`KismetMathLibrary.FClamp` (+ (`self.health`) amount) 0.0 (`self.maxHealth`))))
  (`KismetSystemLibrary.PrintString` (`KismetStringLibrary.Conv_DoubleToString` _output_get))
  (set `self.healing` true)
  (`/Engine/EditorBlueprintResources/StandardMacros.IsValid` null
    (:`Is Valid`
      (`GameplayStatics.PlaySoundAtLocation` "/Game/refereance/firstperson_bannasa/audio/playerHeal.playerHeal" _returnvalue (struct) (`self.volume mult`) 1.0 0.0 null null null null)
      (`NiagaraFunctionLibrary.SpawnSystemAtLocation` "/Game/ART/particles/FXS_playerHeal.FXS_playerHeal" _returnvalue)
      (set `self.healing` true))))

(fn `kill`)

(fn `playFX`
  (bind _sound (`self.Sound`))
  (bind _returnvalue (`Actor.K2_GetActorLocation` (`self.owner`)))
  (`/Engine/EditorBlueprintResources/StandardMacros.IsValid` _sound
    (:`Is Valid`
      (`GameplayStatics.PlaySoundAtLocation` _sound _returnvalue (struct) (`self.volume mult`) 1.0 0.0 null null null null)
      (`NiagaraFunctionLibrary.SpawnSystemAtLocation` (`self.System Template`) _returnvalue))))

(fn `take damage`)