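; Stamina component that tracks a clamped pool, filled at BeginPlay and regenerated by a looping timer instead of Tick.
; Spending subtracts stamina and pauses regeneration, which a second named timer resumes.
; The resume delay is the configured spend pause below a low threshold, otherwise a fixed one.
; That resume timer loops, so it keeps unpausing regeneration, and the pause's Duration input is unused.
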(event `self.ReceiveBeginPlay`
  (set `self.stamina` (`self.MaxStamina`))
  (bind _returnvalue (`KismetSystemLibrary.K2_SetTimer` null "Tick Stamina" (`self.staminaTickFrequency`) true))
  (set `self.staminaTickTimer` _returnvalue))

(fn `pauseTickStamina`
  (params (duration :type "Float (double-precision)"))
  (`KismetSystemLibrary.K2_PauseTimerHandle` (`self.staminaTickTimer`))
  (if (> 2.0 (`self.stamina`))
    (`KismetSystemLibrary.K2_SetTimer` null "StartTickStamina" (`self.staminaSpendPauseDuration`) true)
    (else
      (`KismetSystemLibrary.K2_SetTimer` null "StartTickStamina" 1.0 true))))

(fn `spendStamina`
  (params (amount :type "Float (double-precision)"))
  (if (> amount 0.0)
    (set `self.stamina` (`KismetMathLibrary.FClamp` (- (`self.stamina`) amount) 0.0 (`self.MaxStamina`)))
    (`self.pauseTickStamina` (`self.staminaSpendPauseDuration`))))

(fn `StartTickStamina`
  (`KismetSystemLibrary.K2_UnPauseTimerHandle` (`self.staminaTickTimer`)))

(fn `stopTickStamina`
  (`KismetSystemLibrary.K2_PauseTimerHandle` (`self.staminaTickTimer`)))

(fn `Tick Stamina`
  (set `self.stamina` (`KismetMathLibrary.FClamp` (+ (`self.stamina`) (* (`self.StaminaRegenPerSec`) (`self.staminaTickFrequency`))) 0.0 (`self.MaxStamina`))))