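; A collectable pickup that grants one unit of currency to the local player on contact.
; On collision overlap it checks that the other actor is player 0's third-person character.
; It then increments CurrencyCount on that player's BP_thirdPersonPlayerState and destroys itself, with debug prints for the overlap, new count and failed state cast.
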(event `self.collision.OnComponentBeginOverlap`
  (params (OverlappedComponent :type "PrimitiveComponent Object Reference") (OtherActor :type "Actor Object Reference") (OtherComp :type "PrimitiveComponent Object Reference") (OtherBodyIndex :type Integer) (bFromSweep :type Boolean) (SweepResult :type "HitResult Structure (by ref)"))
  (bind _asbp_third_person_character (cast `/Game/Blueprints/Characters/3rd_person_Blueprints/BP_ThirdPersonCharacter` (`GameplayStatics.GetPlayerPawn` 0)))
  (if (== OtherActor _asbp_third_person_character)
    (`KismetSystemLibrary.PrintString` "overlap 3rd")
    (bind _asbp_third_person_player_state (cast `/Game/Blueprints/Characters/3rd_person_Blueprints/BP_thirdPersonPlayerState` (`GameplayStatics.GetPlayerState` 0))
      (:`then`
        (bind _output_get (set `/Game/Blueprints/Characters/3rd_person_Blueprints/BP_thirdPersonPlayerState.currency count` (+ 1 (`/Game/Blueprints/Characters/3rd_person_Blueprints/BP_thirdPersonPlayerState.currency count` _asbp_third_person_player_state)) _asbp_third_person_player_state))
        (`KismetSystemLibrary.PrintString` (`KismetStringLibrary.Conv_IntToString` _output_get))
        (`self.K2_DestroyActor`))
      (:`CastFailed`
        (`KismetSystemLibrary.PrintString` "state cast error")))))

(fn `UserConstructionScript`)