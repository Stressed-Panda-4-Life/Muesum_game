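; BP_FlameCircle is a flame circle hazard actor that grows and damages actors.
; On BeginPlay it enables collision on two cylinders and plays a timeline that multiplies Cylinder's scale each update, widening it faster than it grows in height.
; Damage fires when an actor stops overlapping Cylinder1, not on entry, and skips actors implementing BPI_fire_resitant.
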(event `self.ReceiveBeginPlay`
  (`PrimitiveComponent.SetCollisionEnabled` (`self.Cylinder`) "QueryAndPhysics")
  (`PrimitiveComponent.SetCollisionEnabled` (`self.Cylinder1`) "QueryAndPhysics")
  (`Timeline|Timeline`
    (:`Update`
      (`SceneComponent.SetRelativeScale3D` (`self.Cylinder`) (* (`SceneComponent.RelativeScale3D` (`self.Cylinder`)) (1.01 1.01 1.001))))))

(event `self.Cylinder1.OnComponentEndOverlap`
  (params (OverlappedComponent :type "PrimitiveComponent Object Reference") (OtherActor :type "Actor Object Reference") (OtherComp :type "PrimitiveComponent Object Reference") (OtherBodyIndex :type Integer))
  (if (not (`KismetSystemLibrary.DoesImplementInterface` OtherActor "/Game/Blueprints/Input/BPI_fire_resitant.BPI_fire_resitant_C"))
    (`GameplayStatics.ApplyDamage` OtherActor (`self.Base Damage`))))

(fn `UserConstructionScript`)